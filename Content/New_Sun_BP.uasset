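; Sun actor that continuously spawns short-lived bright storm meshes at random points around itself.
; Tick drives three DoOnce-gated slots, each spawning a storm, animating its AlphaInLife material parameter by Timeline, then destroying it and resetting.
; Storms rotates a reference sphere's offset randomly for placement, scales the mesh by lifetime and assigns two dynamic materials.
; Scale, Timeline rate and destroy delay each roll their own random duration around BrightStormAvgLife.
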(event EventBeginPlay)

(event Collision|EventActorBeginOverlap
  (params (OtherActor :type Actor%20Object%20Reference)))

(event EventTick
  (params (DeltaSeconds :type Float%20%28single-precision%29))
  (bind _returnvalue (Math|Random|RandomFloat))
  (bind _returnvalue_2 (Math|Random|RandomFloat))
  (bind _returnvalue_3 (Math|Random|RandomFloat))
  (bind _brightstormavglife (Variables|Default|GetBrightStormAvgLife))
  (bind _brightstormavglife_2 (Variables|Default|GetBrightStormAvgLife))
  (bind _brightstormavglife_3 (Variables|Default|GetBrightStormAvgLife))
  (bind _returnvalue_4 (* _brightstormavglife _returnvalue))
  (bind _returnvalue_5 (* _brightstormavglife_2 _returnvalue_2))
  (bind _returnvalue_6 (* _brightstormavglife_3 _returnvalue_3))
  (bind _returnvalue_7 (+ _returnvalue_4 7.0))
  (bind _returnvalue_8 (+ _returnvalue_5 7.0))
  (bind _returnvalue_9 (+ _returnvalue_6 7.0))
  (Utilities|FlowControl|Sequence
    (:then_0
      (Utilities|FlowControl|DoOnce false :!label _label
        (:Completed
          (bind _stormcreated (CallFunction|Storms _returnvalue_8))
          (Components|Timeline|SetPlayRate (Variables|Default|GetTimeline_0) (/ 1.0 _returnvalue_8))
          (bind _time (Timeline|Timeline_0 PlayFromStart)
            (:Update
              (Utilities|IsValid _stormcreated
                (:Is%20Valid
                  (Rendering|Material|SetScalarParameterValueonMaterials _stormcreated "AlphaInLife" _time)
                  (Utilities|FlowControl|Delay _returnvalue_8)
                  (Components|DestroyComponent _stormcreated)
                  (Utilities|FlowControl|Delay 1.0)
                  (goto _label Reset))))))))
    (:then_1
      (Utilities|FlowControl|DoOnce false :!label _label_2
        (:Completed
          (bind _stormcreated_2 (CallFunction|Storms _returnvalue_9))
          (Components|Timeline|SetPlayRate (Variables|Default|GetTimeline_1) (/ 1.0 _returnvalue_9))
          (bind _time_2 (Timeline|Timeline_1 PlayFromStart)
            (:Update
              (Utilities|IsValid _stormcreated_2
                (:Is%20Valid
                  (Rendering|Material|SetScalarParameterValueonMaterials _stormcreated_2 "AlphaInLife" _time_2)
                  (Utilities|FlowControl|Delay _returnvalue_9)
                  (Components|DestroyComponent _stormcreated_2)
                  (Utilities|FlowControl|Delay 1.0)
                  (goto _label_2 Reset))))))))
    (:then_2
      (Utilities|FlowControl|DoOnce false :!label _label_3
        (:Completed
          (bind _stormcreated_3 (CallFunction|Storms _returnvalue_7))
          (Components|Timeline|SetPlayRate (Variables|Default|GetTimeline_2) (/ 1.0 _returnvalue_7))
          (bind _time_3 (Timeline|Timeline_2 PlayFromStart)
            (:Update
              (Utilities|IsValid _stormcreated_3
                (:Is%20Valid
                  (Rendering|Material|SetScalarParameterValueonMaterials _stormcreated_3 "AlphaInLife" _time_3)
                  (Utilities|FlowControl|Delay _returnvalue_7)
                  (Components|DestroyComponent _stormcreated_3)
                  (Utilities|FlowControl|Delay 1.0)
                  (goto _label_3 Reset))))))))))

(fn ConstructionScript)

(fn Storms
  (params (LifeTime :type Float%20%28single-precision%29))
  (bind _returnvalue (Math|Random|RandomRotator false))
  (bind _returnvalue_2 (/ LifeTime 1e+01))
  (bind _returnvalue_3 (AddComponent|AddStaticMeshComponent false (Math|Transform|MakeTransform (Math|Vector|RotateVector (.Location (Math|Transform|BreakTransform (Transformation|GetRelativeTransform (Variables|Default|GetBrightStorms_pSphere1)))) _returnvalue) _returnvalue (Math|Vector|MakeVector _returnvalue_2 _returnvalue_2 _returnvalue_2))))
  (bind _returnvalue_4 (Rendering|Material|CreateDynamicMaterialInstance _returnvalue_3 0 "/Game/M_BrightStormBase.M_BrightStormBase" :!class /Script/Engine.PrimitiveComponent))
  (bind _returnvalue_5 (Rendering|Material|CreateDynamicMaterialInstance _returnvalue_3 1 "/Game/M_BrightStorm.M_BrightStorm" :!class /Script/Engine.PrimitiveComponent))
  (Rendering|Material|SetMaterial _returnvalue_3 1 _returnvalue_5)
  (Rendering|Material|SetMaterial _returnvalue_3 0 _returnvalue_4)
  (return _returnvalue_3))